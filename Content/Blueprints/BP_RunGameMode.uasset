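; Game mode for a tile-based runner that creates the game UI and lays ten default floor tiles at BeginPlay.
; AddFloorTile chains the track by spawning each tile at the spawn point returned by the previous one and counting it in ItemDelta.
; For non-default tiles, RandomTile compares TileDelta to a random threshold to pick a random straight or corner piece, spacing out turns and resetting the count after each corner.
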(event EventBeginPlay
  (bind _returnvalue (UserInterface|CreateWidget "/Game/Blueprints/GameUI.GameUI_C"))
  (UserInterface|Viewport|AddtoViewport _returnvalue 0)
  (for _index (range 1 10)
    (CallFunction|AddFloorTile true)))

(fn ConstructionScript)

(fn AddFloorTile
  (params (IsDefault :type Boolean))
  (Utilities|FlowControl|Sequence
    (:then_0
      (if IsDefault
        (CallFunction|AddTileDelta)
        (else
          (|RandomTile))))
    (:then_1
      (bind _returnvalue (Game|SpawnActorfromClass (LocalVariables|GetTileClass) (Variables|Default|GetSpawnPoint) "Undefined" 0 0))
      (bind _point (Default|GetSpawnPoint _returnvalue))
      (Variables|Default|SetSpawnPoint _point)
      (Variables|Default|SetItemDelta (+ (Variables|Default|GetItemDelta) 1)))))

(fn AddTileDelta
  (Variables|Default|SetTileDelta (+ (Variables|Default|GetTileDelta) 1)))