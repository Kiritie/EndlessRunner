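; Player character for an endless runner that auto-runs forward, strafes, jumps and tracks coins and distance.
; When CanTurn allows, turn input shifts a target yaw 90 degrees, and Tick interpolates control rotation toward it.
; Head-on Building hits or falling below the last floor position cause death, then a timeline drives ReliveProgress before restarting the level.
; Magnet and shield pickups toggle component visibility and expire on Tick-driven countdowns.
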(event OnComponentHit(CapsuleComponent)
  (params (HitComponent :type Primitive%20Component%20Object%20Reference) (OtherActor :type Actor%20Object%20Reference) (OtherComp :type Primitive%20Component%20Object%20Reference) (NormalImpulse :type Vector :default "0, 0, 0") (Hit :type Hit%20Result%20Structure%20%28by%20ref%29))
  ;[1 1 1] 碰撞检测
  (if (and (Utilities|Name|Equal(Name) (Utilities|Array|Get(acopy) (Variables|/Script/Engine.ActorComponent|GetComponentTags OtherComp)) "Building") (Math|Float|NearlyEqual(Float) (Math|Vector|DotProduct (Math|Vector|GetForwardVector (Variables|Default|GetDesiredRotation)) (.normal Hit)) -1.0 0.01))
    (CallFunction|Death)))

(event Custom|TurnCorner
  (bind _returnvalue (Pawn|GetControlRotation :!class /Script/Engine.Pawn))
  (bind _desiredrotation (Variables|Default|GetDesiredRotation))
  ;[1 1 1] 选择到目标角度
  (if (Utilities|Enum|NotEqual(Enum) _returnvalue _desiredrotation)
    (Pawn|SetControlRotation (Pawn|GetController) (Math|Interpolation|RInterpTo _returnvalue _desiredrotation (Utilities|Time|GetWorldDeltaSeconds) (Variables|Default|GetTurnSpeed)))))

(event Custom|Death
  (bind _returnvalue (Transformation|GetActorLocation))
  ;[1 1 1] 死亡
  (if (not (Variables|Default|GetIsDead))
    (Variables|Default|SetIsDead true)
    (Input|DisableInput 0)
    (Effects|SpawnEmitteratLocation "/Game/StarterContent/Particles/P_Explosion.P_Explosion" _returnvalue)
    (Audio|PlaySoundatLocation "/Game/StarterContent/Audio/Explosion_Cue.Explosion_Cue" _returnvalue)
    (Rendering|SetVisibility (Variables|Character|GetMesh) false true)
    (Pawn|Components|CharacterMovement|DisableMovement (Variables|Character|GetCharacterMovement))
    (CallFunction|StartRelive)))

(event Custom|UpdateItemsDuration
  (params (DeltaTime :type Float%20%28single-precision%29))
  ;[1 1 1] 更新道具持续时间
  (CallFunction|UpdateMagentDuration DeltaTime)
  (CallFunction|UpdateShieldDuration DeltaTime))

(event Custom|StartRelive
  ;[1 1 1] 执行重生
  (bind _progress (Timeline|ReliveTimeline Play)
    (:Update
      (Variables|Default|SetReliveProgress _progress))
    (:Finished
      (Development|ExecuteConsoleCommand "RestartLevel"))))

(event Custom|FallingDeadCheck
  ;[1 1 1] 摔死检测
  (if (AI|Components|NavMovement|IsFalling (Variables|Character|GetCharacterMovement))
    (if (> (.Z (Math|Vector|BreakVector (- (Variables|Default|GetLastFloorPos) (Transformation|GetActorLocation)))) 2e+02)
      (Variables|Default|SetIsDead true)
      (CallFunction|StartRelive))))

(event EventBeginPlay
  ;[1 1 1] 初始化角色
  (Variables|Default|SetDesiredRotation (Pawn|GetControlRotation :!class /Script/Engine.Pawn))
  (CallFunction|SetMagnetVisibility false)
  (CallFunction|SetShieldVisibility false))

(event EventTick
  (params (DeltaSeconds :type Float%20%28single-precision%29))
  ;[1 1 1] 移动控制
  (if (not (Variables|Default|GetIsDead))
    (CallFunction|UpdateItemsDuration DeltaSeconds)
    (CallFunction|TurnCorner)
    (CallFunction|FallingDeadCheck)
    (CallFunction|UpdateDistance)
    (Pawn|Input|AddMovementInput (Math|Vector|GetForwardVector (Math|Rotator|MakeRotator 0.0 0.0 (.Yaw (Math|Rotator|BreakRotator (Pawn|GetControlRotation :!class /Script/Engine.Pawn))))) 1.0 false)))

(event Input|ActionEvents|InputActionJump
  (params (Key :type Key%20Structure :default "AnyKey"))
  ;[1 1 1] 跳跃
  (:Pressed
    (Character|Jump))
  (:Released
    (Character|StopJumping)))

(event Input|ActionEvents|InputActionTurnLeft
  (params (Key :type Key%20Structure :default "AnyKey"))
  ;[1 1 1] 设置目标角度
  (:Pressed
    (if (Variables|Default|GetCanTurn)
      (Variables|Default|SetDesiredRotation (Math|Rotator|CombineRotators (Variables|Default|GetDesiredRotation) "0,-90.000000, 0"))
      (Variables|Default|SetCanTurn false))))

(event Input|ActionEvents|InputActionTurnRight
  (params (Key :type Key%20Structure :default "AnyKey"))
  ;[1 1 1] 设置目标角度
  (:Pressed
    (if (Variables|Default|GetCanTurn)
      (Variables|Default|SetDesiredRotation (Math|Rotator|CombineRotators (Variables|Default|GetDesiredRotation) "0,90.000000, 0"))
      (Variables|Default|SetCanTurn false))))

(event Input|AxisEvents|InputAxisMoveRight
  (params (AxisValue :type Float%20%28single-precision%29))
  ;[1 1 1] 移动控制
  (Pawn|Input|AddMovementInput (Math|Vector|GetRightVector (Math|Rotator|MakeRotator 0.0 0.0 (.Yaw (Math|Rotator|BreakRotator (Pawn|GetControlRotation :!class /Script/Engine.Pawn))))) AxisValue false))

(fn ConstructionScript)

(fn AddCoin
  (Variables|Default|SetCoinCount (+ (Variables|Default|GetCoinCount) 1)))

(fn UpdateDistance
  (bind _returnvalue (Transformation|GetVelocity))
  (Variables|Default|SetDistance (+ (Variables|Default|GetDistance) (* (Math|Vector|VectorLength (Math|Vector|MakeVector (.x _returnvalue) (.y _returnvalue) 0.0)) (Utilities|Time|GetWorldDeltaSeconds)))))

(fn UpdateMagentDuration
  (params (DeltaTime :type Float%20%28single-precision%29))
  (if (Variables|Default|GetUsingMagnet)
    (Variables|Default|SetMagnetDuration (- (Variables|Default|GetMagnetDuration) DeltaTime))
    (if (<= (Variables|Default|GetMagnetDuration) 0.0)
      (Variables|Default|SetUsingMagnet false)
      (CallFunction|SetMagnetVisibility false))))

(fn UseMagnet
  (Variables|Default|SetUsingMagnet true)
  (Variables|Default|SetMagnetDuration (Variables|Default|GetBaseMagnetDuration))
  (CallFunction|SetMagnetVisibility true))

(fn SetMagnetVisibility
  (params (IsVisible :type Boolean))
  (Rendering|SetVisibility (Variables|Default|GetMagnet) IsVisible true))

(fn SetShieldVisibility
  (params (IsVisible :type Boolean))
  (Rendering|SetVisibility (Variables|Default|GetShield) IsVisible true))

(fn UseShield
  (Variables|Default|SetUsingShield true)
  (Variables|Default|SetShieldDuration (Variables|Default|GetBaseShieldDuration))
  (CallFunction|SetShieldVisibility true))

(fn UpdateShieldDuration
  (params (DeltaTime :type Float%20%28single-precision%29))
  (if (Variables|Default|GetUsingShield)
    (Variables|Default|SetShieldDuration (- (Variables|Default|GetShieldDuration) DeltaTime))
    (if (<= (Variables|Default|GetShieldDuration) 0.0)
      (Variables|Default|SetUsingShield false)
      (CallFunction|SetShieldVisibility false))))