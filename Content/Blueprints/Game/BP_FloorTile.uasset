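; Endless-runner floor tile that randomly populates itself and exposes a spawn point transform.
; If CanSpawnItems is set, the construction script randomly picks blockers, coins or an item gated by the game mode's ItemDelta, placed as child actors within box extents.
; When BP_RunCharacter hits the end trigger, the tile records its location as LastFloorPos, requests another tile from BP_RunGameMode, then destroys itself after a delay unless the runner is dead.
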(event OnComponentBeginOverlap(EndTirgger)
  (params (OverlappedComponent :type Primitive%20Component%20Object%20Reference) (OtherActor :type Actor%20Object%20Reference) (OtherComp :type Primitive%20Component%20Object%20Reference) (OtherBodyIndex :type Integer) (bFromSweep :type Boolean) (SweepResult :type Hit%20Result%20Structure%20%28by%20ref%29))
  (bind _asbp_run_character (Utilities|Casting|CastToBP_RunCharacter OtherActor))
  (Variables|/Game/Blueprints/Character/BP_RunCharacter.BP_RunCharacter_C|SetLastFloorPos _asbp_run_character (Transformation|GetActorLocation))
  (bind _asbp_run_game_mode (Utilities|Casting|CastToBP_RunGameMode (Game|GetGameMode)))
  (Default|AddFloorTile _asbp_run_game_mode false)
  (Utilities|FlowControl|Delay 2.0)
  (if (not (Variables|/Game/Blueprints/Character/BP_RunCharacter.BP_RunCharacter_C|GetIsDead _asbp_run_character))
    (Actor|DestroyActor)))

(event EventBeginPlay)

(event Collision|EventActorBeginOverlap
  (params (OtherActor :type Actor%20Object%20Reference)))

(event EventTick
  (params (DeltaSeconds :type Float%20%28single-precision%29)))

(fn ConstructionScript
  (bind _returnvalue (Math|Random|RandomIntegerinRange 1 10))
  (if (Variables|Default|GetCanSpawnItems)
    (LocalVariables|SetTempNum _returnvalue)
    (if (<= _returnvalue 4)
      (CallFunction|SpawnBlocker)
      (elif (<= _returnvalue 8)
        (CallFunction|SpawnCoins)
        (elif true
          (CallFunction|SpawnItem))))))

(fn GetSpawnPoint
  (return (Transformation|GetWorldTransform (Variables|Default|GetSpawnPoint))))

(fn SpawnBlocker
  (bind _blockerextent (Variables|Default|GetBlockerExtent))
  (bind _blockers (Variables|Default|GetBlockers))
  (bind _blockercountrange (Variables|Default|GetBlockerCountRange))
  (bind _blockerscalerange (Variables|Default|GetBlockerScaleRange))
  (for _index (range 1 (Math|Random|RandomIntegerinRange (Utilities|Array|Get(acopy) _blockercountrange) (Utilities|Array|Get(acopy) _blockercountrange 1)))
    (bind _returnvalue (AddComponent|AddChildActorComponent false (Math|Transform|MakeTransform (Math|Random|RandomPointinBoundingBox (Variables|/Script/Engine.SceneComponent|GetRelativeLocation _blockerextent) (Variables|/Script/Engine.BoxComponent|GetBoxExtent _blockerextent)) "0, 0, 0" (* (Math|Vector|MakeVector 1.0 1.0 1.0) (Math|Random|RandomFloatinRange (Utilities|Array|Get(acopy) _blockerscalerange) (Utilities|Array|Get(acopy) _blockerscalerange 1))))))
    (ChildActorComponent|SetChildActorClass _returnvalue (Utilities|Array|Get(acopy) _blockers (Math|Random|RandomInteger (Utilities|Array|Length _blockers))))))

(fn SpawnCoins
  (bind _itemextent (Variables|Default|GetItemExtent))
  (bind _coincountrange (Variables|Default|GetCoinCountRange))
  (for _index (range 1 (Math|Random|RandomIntegerinRange (Utilities|Array|Get(acopy) _coincountrange) (Utilities|Array|Get(acopy) _coincountrange 1)))
    (AddComponent|AddChildActorComponent false (Math|Conversions|ToTransform(Vector) (Math|Random|RandomPointinBoundingBox (Variables|/Script/Engine.SceneComponent|GetRelativeLocation _itemextent) (Variables|/Script/Engine.BoxComponent|GetBoxExtent _itemextent))))))

(fn SpawnItem
  (bind _itemextent (Variables|Default|GetItemExtent))
  (bind _items (Variables|Default|GetItems))
  (bind _asbp_run_game_mode (Utilities|Casting|CastToBP_RunGameMode (Game|GetGameMode)))
  (if (>= (Variables|/Game/Blueprints/BP_RunGameMode.BP_RunGameMode_C|GetItemDelta _asbp_run_game_mode) (Math|Random|RandomIntegerinRange 15 20))
    (Variables|/Game/Blueprints/BP_RunGameMode.BP_RunGameMode_C|SetItemDelta _asbp_run_game_mode 0)
    (bind _returnvalue (AddComponent|AddChildActorComponent false (Math|Conversions|ToTransform(Vector) (Math|Random|RandomPointinBoundingBox (Variables|/Script/Engine.SceneComponent|GetRelativeLocation _itemextent) (Variables|/Script/Engine.BoxComponent|GetBoxExtent _itemextent)))))
    (ChildActorComponent|SetChildActorClass _returnvalue (Utilities|Array|Get(acopy) _items (Math|Random|RandomInteger (Utilities|Array|Length _items))))))