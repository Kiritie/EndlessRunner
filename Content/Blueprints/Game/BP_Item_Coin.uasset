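; BP_Item_Coin is a coin pickup that adds a coin to the character that collects it.
; It caches the player's BP_RunCharacter on BeginPlay and handles collection through the OnPickUp event, which calls AddCoin.
; While the player's magnet is active and the coin is within magnet range, Tick pulls it toward the player with VInterpTo, without sweeping.
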(event EventBeginPlay
  (bind _asbp_run_character (Utilities|Casting|CastToBP_RunCharacter (Game|GetPlayerCharacter 0)))
  (Variables|Default|SetPlayer _asbp_run_character))

(event EventOnPickUp
  (params (Character :type BP%20Run%20Character%20Object%20Reference))
  (Default|AddCoin Character))

(event EventTick
  (params (DeltaSeconds :type Float%20%28single-precision%29))
  (bind _player (Variables|Default|GetPlayer))
  ;[1 1 1] 向玩家移动
  (if (and (Variables|/Game/Blueprints/Character/BP_RunCharacter.BP_RunCharacter_C|GetUsingMagnet _player) (<= (Transformation|GetDistanceTo _player) (Variables|/Game/Blueprints/Character/BP_RunCharacter.BP_RunCharacter_C|GetMagnetRange _player)))
    (Transformation|SetActorLocation (Math|Interpolation|VInterpTo (Transformation|GetActorLocation) (Transformation|GetActorLocation _player) DeltaSeconds 15.0) false false)))

(fn ConstructionScript
  (|CallParentFunction))