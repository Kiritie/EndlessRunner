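; Single floor tile variant that places itself at a randomly chosen race point along the Y axis.
; On construction, SetRacePoint picks a random RacePoints entry as RaceYPoint and shifts Floor, ItemExtent and BlockerExtent to that Y, keeping their X and Z.
; The parent construction script runs afterwards, so it sees the components already repositioned.
; The event graph holds no active logic.
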(event EventBeginPlay)

(event Collision|EventActorBeginOverlap
  (params (OtherActor :type Actor%20Object%20Reference)))

(event EventTick
  (params (DeltaSeconds :type Float%20%28single-precision%29)))

(fn ConstructionScript
  (CallFunction|SetRacePoint)
  (|CallParentFunction))

(fn SetRacePoint
  (bind _blockerextent (Variables|Default|GetBlockerExtent))
  (bind _racepoints (Variables|Default|GetRacePoints))
  (bind _floor (Variables|Default|GetFloor))
  (bind _itemextent (Variables|Default|GetItemExtent))
  (bind _relativelocation (Variables|/Script/Engine.SceneComponent|GetRelativeLocation _blockerextent))
  (bind _relativelocation_2 (Variables|/Script/Engine.SceneComponent|GetRelativeLocation _floor))
  (bind _relativelocation_3 (Variables|/Script/Engine.SceneComponent|GetRelativeLocation _itemextent))
  (LocalVariables|SetRaceYPoint (Utilities|Array|Get(acopy) _racepoints (Math|Random|RandomInteger (Utilities|Array|Length _racepoints))))
  (Utilities|FlowControl|Sequence
    (:then_0
      (Transformation|SetRelativeLocation _floor (Math|Vector|MakeVector (.x _relativelocation_2) (LocalVariables|GetRaceYPoint) (.z _relativelocation_2)) false false))
    (:then_1
      (Transformation|SetRelativeLocation _itemextent (Math|Vector|MakeVector (.x _relativelocation_3) (LocalVariables|GetRaceYPoint) (.z _relativelocation_3)) false false))
    (:then_2
      (Transformation|SetRelativeLocation _blockerextent (Math|Vector|MakeVector (.x _relativelocation) (LocalVariables|GetRaceYPoint) (.z _relativelocation)) false false))))